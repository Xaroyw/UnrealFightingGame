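; Playable 2D fighter character for a local two-player fighting game, with movement along one axis, jumping, ground and air attacks, and blocking.
; Player 2's inputs are caught here and forwarded to the second player pawn, which gets a tinted sprite.
; Attack events damage actors overlapping hitboxes, while animation jumps and flipbook-length delays lock walking.
; Blocking reduces incoming damage; death disables both pawns' input and calls the winner event.
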(event `LoadControls`
  (bind _asplayer_controller (cast `PlayerController` (`self.GetController`) :!label _label))
  (bind _returnvalue (pcsubsystem `EnhancedInputLocalPlayerSubsystem` _asplayer_controller))
  (`/Engine/EditorBlueprintResources/StandardMacros.IsValid` _returnvalue
    (:`Is Valid`
      (`EnhancedInputSubsystemInterface.AddMappingContext` _returnvalue "/Game/Controls/Fighting_IMC.Fighting_IMC" 0 (struct))
      (set `self.Playerspeed` (`MovementComponent.GetMaxSpeed` (`self.CharacterMovement`)))
      (set `self.PlayerMaxHealth` (`self.Playerhealth`)))))

(event `self.ReceiveBeginPlay`
  (goto _label))

(event `EnhancedInput|/Game/Controls/move_IA`
  (params (ActionValue :type "Float (double-precision)") (ElapsedSeconds :type "Float (double-precision)") (TriggeredSeconds :type "Float (double-precision)") (InputAction :type "InputAction Object Reference" :default "/Game/Controls/move_IA.move_IA"))
  ;[1 1 1] Hadle movement and jumping
  (:`Triggered`
    (`self.AddMovementInput` (1.0 0.0 0.0) ActionValue)))

(event `Player2jump`
  ;[1 1 1] Hadle movement and jumping
  (`self.Checkifblocking` :!label _label_2
    (:`else`
      _)
    (:`then`
      _))
  (`self.Jump`))

(event `EnhancedInput|/Game/Controls/Jump_IA`
  (params (ActionValue :type Boolean) (ElapsedSeconds :type "Float (double-precision)") (TriggeredSeconds :type "Float (double-precision)") (InputAction :type "InputAction Object Reference" :default "/Game/Controls/Jump_IA.Jump_IA"))
  ;[1 1 1] Hadle movement and jumping
  (:`Started`
    (goto _label_2))
  (:`Completed`
    (`self.StopJumping`)))

(event `AirAttack`
  ;[1 1 1] Handle dealing damage
  (for _array_element (`PrimitiveComponent.GetOverlappingActors` (`self.airbox`) null)
    (if (!= _array_element self)
      (`GameplayStatics.ApplyDamage` _array_element (`self.Base Damage`)))))

(event `Attack`
  ;[1 1 1] Handle dealing damage
  (for _array_element (`PrimitiveComponent.GetOverlappingActors` (`self.attackbox`) null)
    (if (!= _array_element self)
      (`GameplayStatics.ApplyDamage` _array_element (`self.Base Damage`)))))

(event `Blockplayer2`
  ;[1 1 1] Blocking system
  (if (not (`NavMovementComponent.IsFalling` (`self.CharacterMovement`))) :!label _label_3
    (set `self.IsBlocking?` true)
    (set `CharacterMovementComponent.MaxWalkSpeed` 0.0 (`self.CharacterMovement`))))

(event `EnhancedInput|/Game/Controls/Block_IA`
  (params (ActionValue :type Boolean) (ElapsedSeconds :type "Float (double-precision)") (TriggeredSeconds :type "Float (double-precision)") (InputAction :type "InputAction Object Reference" :default "/Game/Controls/Block_IA.Block_IA"))
  ;[1 1 1] Blocking system
  (:`Started`
    (goto _label_3))
  (:`Completed`
    (set `self.IsBlocking?` false :!label _label_4)
    (set `CharacterMovementComponent.MaxWalkSpeed` (`self.Playerspeed`) (`self.CharacterMovement`))))

(event `Stopblockingplayer2`
  ;[1 1 1] Blocking system
  (goto _label_4))

(event `Player2Atk`
  ;[1 1 1] Attack system
  (`/Engine/EditorBlueprintResources/StandardMacros.DoOnce` false :!label _label_5
    (:`Completed`
      (`self.Checkifblocking`
        (:`else`
          _)
        (:`then`
          _))
      (set `CharacterMovementComponent.MaxWalkSpeed` 0.0 (`self.CharacterMovement`))
      (if (`NavMovementComponent.IsFalling` (`self.CharacterMovement`))
        ;;[1 1 1] Air attack
        (`PaperZDAnimInstance.JumpToNode` (`PaperZDAnimationComponent.AnimInstance` (`self.AnimationComponent`)) "AirAttack" "None")
        (`KismetSystemLibrary.Delay` (- (`PaperFlipbookComponent.GetFlipbookLength` (`self.Sprite`)) 0.25))
        (else
          ;;[1 1 1] Ground attack
          (`PaperZDAnimInstance.JumpToNode` (`PaperZDAnimationComponent.AnimInstance` (`self.AnimationComponent`)) "Attack" "None")
          (`KismetSystemLibrary.Delay` (- (`PaperFlipbookComponent.GetFlipbookLength` (`self.Sprite`)) 0.25))))
      (set `CharacterMovementComponent.MaxWalkSpeed` (`self.Playerspeed`) (`self.CharacterMovement`))
      (goto _label_5 :!via `Reset`))))

(event `EnhancedInput|/Game/Controls/attack_IA`
  (params (ActionValue :type Boolean) (ElapsedSeconds :type "Float (double-precision)") (TriggeredSeconds :type "Float (double-precision)") (InputAction :type "InputAction Object Reference" :default "/Game/Controls/attack_IA.attack_IA"))
  ;[1 1 1] Attack system
  (:`Started`
    (goto _label_5)))

(event `self.ReceiveAnyDamage`
  (params (Damage :type "Float (single-precision)") (DamageType :type "DamageType Object Reference") (InstigatedBy :type "Controller Object Reference") (DamageCauser :type "Actor Object Reference"))
  ;[1 1 1] Handle taking damage
  (bind _output_get (set `self.Playerhealth` (select `bool` (`self.IsBlocking?`) :`false` (- (`self.Playerhealth`) Damage) :`true` (- (`self.Playerhealth`) (/ Damage 5.0)))))
  (`self.Updatehealth`)
  (if (<= _output_get 0.0)
    (`/Engine/EditorBlueprintResources/StandardMacros.DoOnce` false
      (:`Completed`
        (`PaperZDAnimInstance.JumpToNode` (`PaperZDAnimationComponent.AnimInstance` (`self.AnimationComponent`)) "Death" "None")
        (`self.DisableInput` (`GameplayStatics.GetPlayerPawn` 0) null)
        (`self.DisableInput` (`GameplayStatics.GetPlayerPawn` 1) null)
        (`self.Whowon`)))
    (elif (not (`self.IsBlocking?`))
      (`PaperZDAnimInstance.JumpToNode` (`PaperZDAnimationComponent.AnimInstance` (`self.AnimationComponent`)) "damaged" "None")
      (set `CharacterMovementComponent.MaxWalkSpeed` 0.0 (`self.CharacterMovement`))
      (`KismetSystemLibrary.RetriggerableDelay` (- (`PaperFlipbookComponent.GetFlipbookLength` (`self.Sprite`)) 0.3))
      (if (not (`self.IsBlocking?`))
        (set `CharacterMovementComponent.MaxWalkSpeed` (`self.Playerspeed`) (`self.CharacterMovement`))))))

(event `MovePlayer2`
  (params (axisvalue :type "Float (double-precision)"))
  ;[1 1 1] Move Player 2
  (`self.AddMovementInput` (1.0 0.0 0.0) axisvalue))

(event `EnhancedInput|/Game/Controls/MovePlayer2_IA`
  (params (ActionValue :type "Float (double-precision)") (ElapsedSeconds :type "Float (double-precision)") (TriggeredSeconds :type "Float (double-precision)") (InputAction :type "InputAction Object Reference" :default "/Game/Controls/MovePlayer2_IA.MovePlayer2_IA"))
  (bind _player2 (`self.Player2`))
  ;[1 1 1] Move Player 2
  (:`Triggered`
    (`/Engine/EditorBlueprintResources/StandardMacros.IsValid` _player2
      (:`Is Valid`
        (`self.MovePlayer2` _player2 ActionValue))
      (:`Is Not Valid`
        (bind _asplayer_charecter_bp (cast `/Game/blueprint/playerCharecter_BP` (`GameplayStatics.GetPlayerPawn` 1)))
        (bind _output_get (set `self.Player2` _asplayer_charecter_bp))
        (`self.MovePlayer2` _output_get ActionValue)))))

(event `Key|Up`
  (params (Key :type "Key Structure"))
  (bind _player2 (`self.Player2`))
  ;[1 1 1] Move Player 2
  (:`Pressed`
    (`/Engine/EditorBlueprintResources/StandardMacros.IsValid` _player2
      (:`Is Valid`
        (`self.Player2jump` _player2))
      (:`Is Not Valid`
        (bind _asplayer_charecter_bp (cast `/Game/blueprint/playerCharecter_BP` (`GameplayStatics.GetPlayerPawn` 1)))
        (bind _output_get (set `self.Player2` _asplayer_charecter_bp))
        (`self.Player2jump` _output_get)))))

(event `Key|RightShift`
  (params (Key :type "Key Structure"))
  (bind _player2 (`self.Player2`))
  ;[1 1 1] Move Player 2
  (:`Pressed`
    (`/Engine/EditorBlueprintResources/StandardMacros.IsValid` _player2
      (:`Is Valid`
        (`self.Player2Atk` _player2))
      (:`Is Not Valid`
        (bind _asplayer_charecter_bp (cast `/Game/blueprint/playerCharecter_BP` (`GameplayStatics.GetPlayerPawn` 1)))
        (bind _output_get (set `self.Player2` _asplayer_charecter_bp))
        (`self.Player2Atk` _output_get)))))

(event `EnhancedInput|/Game/Controls/BlockPlayer2_IA`
  (params (ActionValue :type Boolean) (ElapsedSeconds :type "Float (double-precision)") (TriggeredSeconds :type "Float (double-precision)") (InputAction :type "InputAction Object Reference" :default "/Game/Controls/BlockPlayer2_IA.BlockPlayer2_IA"))
  ;[1 1 1] Move Player 2
  (:`Started`
    (`/Engine/EditorBlueprintResources/StandardMacros.IsValid` (`self.Player2`)
      (:`Is Valid`
        (`self.Blockplayer2` (`self.Player2`)))
      (:`Is Not Valid`
        (bind _asplayer_charecter_bp (cast `/Game/blueprint/playerCharecter_BP` (`GameplayStatics.GetPlayerPawn` 1)))
        (bind _output_get (set `self.Player2` _asplayer_charecter_bp))
        (`self.Blockplayer2` _output_get))))
  (:`Completed`
    (`/Engine/EditorBlueprintResources/StandardMacros.IsValid` (`self.Player2`)
      (:`Is Valid`
        (`self.Stopblockingplayer2` (`self.Player2`)))
      (:`Is Not Valid`
        (bind _asplayer_charecter_bp_2 (cast `/Game/blueprint/playerCharecter_BP` (`GameplayStatics.GetPlayerPawn` 1)))
        (bind _output_get_2 (set `self.Player2` _asplayer_charecter_bp_2))
        (`self.Stopblockingplayer2` _output_get_2)))))

(fn `UserConstructionScript`
  (if (`self.IsPlayer2?`)
    (`PaperFlipbookComponent.SetSpriteColor` (`self.Sprite`) (struct :`R` 1.0 :`G` 0.986328 :`B` 0.616191 :`A` 1.0))))